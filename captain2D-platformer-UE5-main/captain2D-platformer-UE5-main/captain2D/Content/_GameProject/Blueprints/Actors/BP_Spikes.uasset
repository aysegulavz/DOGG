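; BP_Spikes is a spike hazard actor that damages BP_Player when it overlaps the collision component.
; If CanMove is set, BeginPlay stores the origin and, after a start delay, starts a looping timer that flip-flops a Timeline between play and reverse.
; The Timeline lerps the actor to the world-space HidoutLocation and back, keeping the origin's value on zero axes.
; An all-zero HidoutLocation prints an error instead of moving.
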(event OnComponentBeginOverlap(collisionDamagePlayer)
  (params (OverlappedComponent :type Primitive%20Component%20Object%20Reference) (OtherActor :type Actor%20Object%20Reference) (OtherComp :type Primitive%20Component%20Object%20Reference) (OtherBodyIndex :type Integer) (bFromSweep :type Boolean) (SweepResult :type Hit%20Result%20Structure%20%28by%20ref%29))
  (bind _asbp_player (Utilities|Casting|CastToBP_Player OtherActor))
  (Game|Damage|ApplyDamage _asbp_player (Variables|Default|GetplayerDamageValue) 0 0))

(event Custom|toggleSpike
  (bind _hidoutlocation (Variables|Default|GethidoutLocation))
  (bind _hidoutlocation_2 (Variables|Default|GethidoutLocation))
  (bind _hidoutlocation_3 (Variables|Default|GethidoutLocation))
  (Utilities|FlowControl|FlipFlop
    (:A
      (bind _newtrack_0 (Timeline|Timeline Play)
        (:Update
          (Transformation|SetActorLocation (Math|Vector|Lerp(Vector) (Variables|Default|GetoriginActorWorldLocation) (Math|Vector|MakeVector (select (== (.x _hidoutlocation) 0.0) (.x (Variables|Default|GetoriginActorWorldLocation)) (.x _hidoutlocation)) (select (== (.y _hidoutlocation_2) 0.0) (.y (Variables|Default|GetoriginActorWorldLocation)) (.y _hidoutlocation_2)) (select (== (.z _hidoutlocation_3) 0.0) (.z (Variables|Default|GetoriginActorWorldLocation)) (.z _hidoutlocation_3))) _newtrack_0) false false))))
    (:B
      (Timeline|Timeline Reverse))))

(event Custom|applySpikeMovement
  (if (Variables|Default|GetcanMove?)
    ;[0.9042 0 0.7656] DELETE: only used for debugging
    (if (Utilities|Operators|NotEqual(!=) :A (Variables|Default|GethidoutLocation))
      (Variables|Default|SetoriginActorWorldLocation (Transformation|GetActorLocation))
      (Utilities|FlowControl|Delay (Variables|Default|GetmovementStartDelay%20%28In%20seconds%29))
      (Utilities|Time|SetTimerbyEvent (delegate Custom|toggleSpike) (Variables|Default|GetmovementSwitchTime%20%28In%20Seconds%29) true)
      (else
        (Development|PrintString "ERROR: Define the valid location on the spike hiden" true true "(R=0.000000,G=0.660000,B=1.000000,A=1.000000)" 5.0)))))

(event EventBeginPlay
  (CallFunction|ApplySpikeMovement))

(fn ConstructionScript)