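; Game Instance that keeps the current level number and the player death count across level loads.
; Updating the level increments the number and can optionally open that level at once.
; Levels open by a name built from a base name plus the number, so maps follow a numbered naming scheme.
; A separate event increments the death count.
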(event Custom|updatePlayerDeathCount
  (bind _result (Math|Integer|IncrementInt (Variables|Default|GetamountPlayerDeath))
    (:%20%20
      (Variables|Default|SetamountPlayerDeath _result))))

(event Custom|openLevel
  (params (level :type Integer))
  (Game|OpenLevel(byName) (Utilities|String|StringToName (Utilities|String|Append (Variables|Default|GetlevelsBaseName) (Utilities|String|ToString(Integer) level)))))

(event Custom|updateCurrentLevel
  (params (openTheLevel? :type Boolean))
  (bind _result (Math|Integer|IncrementInt (Variables|Default|GetcurrentLevel))
    (:%20%20
      (bind _output_get (Variables|Default|SetcurrentLevel _result))
      (if openTheLevel?
        (CallFunction|OpenLevel _output_get)))))