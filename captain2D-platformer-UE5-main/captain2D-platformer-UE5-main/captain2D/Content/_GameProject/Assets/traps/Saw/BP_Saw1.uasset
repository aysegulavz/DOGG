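; BP_Saw1 is a saw trap that moves a Paper2D flipbook along a spline and damages the player on overlap.
; On BeginPlay, a timeline scaled by a configurable duration maps its progress to distance along the spline.
; When Loop is set, the timeline's finish re-triggers a FlipFlop that alternates Play and Reverse for back-and-forth motion.
; A collision component applies configurable damage to any overlapping BP_Player.
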(event OnComponentBeginOverlap(collisionDamagePlayer)
  (params (OverlappedComponent :type Primitive%20Component%20Object%20Reference) (OtherActor :type Actor%20Object%20Reference) (OtherComp :type Primitive%20Component%20Object%20Reference) (OtherBodyIndex :type Integer) (bFromSweep :type Boolean) (SweepResult :type Hit%20Result%20Structure%20%28by%20ref%29))
  (bind _asbp_player (Utilities|Casting|CastToBP_Player OtherActor))
  (Game|Damage|ApplyDamage _asbp_player (Variables|Default|GetplayerDamageValue) 0 0))

(event Custom|playSplineMovement
  (bind _spline (Variables|Default|GetSpline))
  (Components|Timeline|SetPlayRate (Variables|Default|GetTimeline_SplineMovement) (/ 0.5 (Variables|Default|GetsplineMovementDuration%20%28In%20Seconds%29)))
  (Utilities|FlowControl|FlipFlop
    (:A
      (bind _duraction (Timeline|Timeline_SplineMovement Play)
        (:Update
          (Transformation|SetWorldLocation (Variables|Default|GetPaperFlipbook) (Spline|GetLocationatDistanceAlongSpline _spline (* _duraction (Spline|GetSplineLength _spline)) "World") false false))
        (:Finished
          ;[1 1 1] If "loop?" is true, the motion will reverse. Otherwise, the actor stops at the last point of the spline
          (if (Variables|Default|Getloop?)
            (CallFunction|PlaySplineMovement)))))
    (:B
      (Timeline|Timeline_SplineMovement Reverse))))

(event EventBeginPlay
  (CallFunction|PlaySplineMovement))

(fn ConstructionScript)